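; Game manager that runs the timed day loop of a mission game with penguin heroes, bird factions, masks and fish currency.
; Timers drive the clock and spawn missions at shuffled spawners; the day ends once time expires and no missions remain active.
; Day end charges level-based fish upkeep, locks or rehires penguins, then pauses via time dilation for the review.
; Faction relations randomize at BeginPlay; mission scoring only prints, and ChangeRelation is an empty stub.
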(event `self.ReceiveBeginPlay`
  (bind _outactors (`GameplayStatics.GetAllActorsOfClass` "/Game/Blueprints/WorldObjects/BP_MissionSpawner.BP_MissionSpawner_C"))
  (set `self.MissionSpawners` _outactors)
  (`self.RandomlyChangeRelations`)
  (`GameplayStatics.SetGlobalTimeDilation` 0.0))

(fn `AddMasks`
  (params (MasksToAdd :type "Array of /Game/Blueprints/Data/E_Masks Enum"))
  (for _array_element MasksToAdd
    (bind _value (`BlueprintMapLibrary.Map_Find` (`/Game/Blueprints/UI/WBP_MaskInventory.EnumToMask` (`/Game/Blueprints/UI/WBP_MainUI.WBP_MaskInventory` (`self.PlayerUI`))) _array_element))
    (bind _result (`/Engine/EditorBlueprintResources/StandardMacros.IncrementInt` (`/Game/Blueprints/UI/WBP_MaskItem.Amount` _value))
      (:`  `
        (`/Game/Blueprints/UI/WBP_MaskItem.SetItemCount` _value _result)))))

(fn `CalculateMission`
  (params (Masks :type "Array of /Game/Blueprints/Data/E_Masks Enum") (Penguins :type "Array of /Game/Blueprints/Data/E_Penguin Enum") (Mission :type "/Game/Blueprints/Data/ST_MissionData Structure"))
  (locals (`L-CompleationPercentage` :type "Float (double-precision)"))
  (bind ((`MajorSolution_12_EC0524D447D1E96047F036B81B3052B6` _majorsolution) (`MinorSolution_14_569F0B8E4560991994FC369CC99F4337` _minorsolution)) (break `/Game/Blueprints/Data/ST_MissionData` Mission))
  (for _array_element (`local.Penguins`)
    (if (`|EnumEquality` _array_element _majorsolution)
      (set `local.L-CompleationPercentage` (+ (`local.L-CompleationPercentage`) 1.5))
      (elif (`|EnumEquality` _array_element _minorsolution)
        (set `local.L-CompleationPercentage` (+ (`local.L-CompleationPercentage`) 1.0))
        (else
          (set `local.L-CompleationPercentage` (+ (`local.L-CompleationPercentage`) 0.5))))))
  (for _array_element_2 (`local.Masks`)
    (set `local.L-CompleationPercentage` (+ (`local.L-CompleationPercentage`) (* (select `/Game/Blueprints/Data/E_Status` (`self.GetRelation` (`.MissionTarget_35_B064C9994A4F7CA83C9762BAEE1FF0B6` (break `/Game/Blueprints/Data/ST_MissionData` (`local.Mission`))) _array_element_2) :`NewEnumerator1` 1.5 :`NewEnumerator2` 1.0 :`NewEnumerator3` 0.5) (select `bool` (`|EnumEquality` _array_element_2 (`.MissionGiver_31_CCAE2BFC4D208B983846BFAD44B6B8F0` (break `/Game/Blueprints/Data/ST_MissionData` (`local.Mission`)))) :`false` 1.0)))))
  (`KismetSystemLibrary.PrintString` (`KismetStringLibrary.Conv_DoubleToString` (/ (`local.L-CompleationPercentage`) (`KismetArrayLibrary.Array_Length` (`local.Penguins`))))))

(fn `CalculateMostAndLeastMissiomTypes`
  (params (MissionsDone :type "Array of /Game/Blueprints/Data/E_Masks Enum"))
  (returns (Greatest :type "/Game/Blueprints/Data/E_Masks Enum") (Lowest :type "/Game/Blueprints/Data/E_Masks Enum"))
  (locals (`L-Counts` :type "Array of Integer") (`L-Int` :type Integer) (`L-Index` :type Integer) (`L-Greatest` :type "/Game/Blueprints/Data/E_Masks Enum") (`L-Lowest` :type "/Game/Blueprints/Data/E_Masks Enum"))
  (for _array_element (`|MakeArray` "NewEnumerator1" "NewEnumerator2" "NewEnumerator3" "NewEnumerator4" "NewEnumerator5" :!type "/Game/Blueprints/Data/E_Masks Enum")
    (set `local.L-Int` 0)
    (for _array_element_2 MissionsDone
      (if (`|EnumEquality` _array_element _array_element_2)
        (`/Engine/EditorBlueprintResources/StandardMacros.IncrementInt` (`local.L-Int`))))
    (`KismetArrayLibrary.Array_Add` (`local.L-Counts`) (`local.L-Int`)))
  (set `local.L-Int` 0)
  (set `local.L-Index` 0)
  (for (_array_element_3 _array_index) (`local.L-Counts`)
    (if (>= _array_element_3 (`local.L-Int`))
      (set `local.L-Int` _array_element_3)
      (set `local.L-Index` _array_index)))
  (set `local.L-Greatest` (`|GetArrayItem` (`|MakeArray` "NewEnumerator1" "NewEnumerator2" "NewEnumerator3" "NewEnumerator4" "NewEnumerator5" :!type "/Game/Blueprints/Data/E_Masks Enum") (`local.L-Index`)))
  (set `local.L-Int` 0)
  (set `local.L-Index` 0)
  (for (_array_element_4 _array_index_2) (`local.L-Counts`)
    (if (<= _array_element_4 (`local.L-Int`))
      (set `local.L-Int` _array_element_4)
      (set `local.L-Index` _array_index_2)))
  (set `local.L-Lowest` (`|GetArrayItem` (`|MakeArray` "NewEnumerator1" "NewEnumerator2" "NewEnumerator3" "NewEnumerator4" "NewEnumerator5" :!type "/Game/Blueprints/Data/E_Masks Enum") (`local.L-Index`)))
  (return (`local.L-Greatest`) (`local.L-Lowest`)))

(fn `CalculateRelationChange`
  (params (Relation :type "/Game/Blueprints/Data/E_Status Enum" :default "NewEnumerator0"))
  (returns (NewRelation :type "/Game/Blueprints/Data/E_Status Enum"))
  (locals (`L-Relation` :type "/Game/Blueprints/Data/E_Status Enum" :default "NewEnumerator0") (`L-RandomValue` :type "Float (double-precision)" :default 0.0))
  (set `local.L-Relation` Relation)
  (set `local.L-RandomValue` (`KismetMathLibrary.RandomFloatInRange` 0.0 100.0))
  (return (cast `/Game/Blueprints/Data/E_Status` (`KismetMathLibrary.Conv_IntToByte` (`KismetMathLibrary.Clamp` (select `bool` (> (`local.L-RandomValue`) 80.0) :`false` (`KismetMathLibrary.Conv_ByteToInt` (`local.L-Relation`)) :`true` (select `bool` (> (`local.L-RandomValue`) 90.0) :`false` (- (`KismetMathLibrary.Conv_ByteToInt` (`local.L-Relation`)) 1) :`true` (+ (`KismetMathLibrary.Conv_ByteToInt` (`local.L-Relation`)) 1))) 1 3)))))

(fn `ChangeRelation`
  (params (RelationsOf :type "/Game/Blueprints/Data/E_Masks Enum" :default "NewEnumerator0") (With :type "/Game/Blueprints/Data/E_Masks Enum" :default "NewEnumerator0") (Amount :type Integer)))

(fn `CheckForEndDay`
  (if (and (<= (`self.ActiveMissionCount`) 0) (not (`KismetSystemLibrary.K2_IsValidTimerHandle` (`self.TotalDayTimer`))))
    (`KismetSystemLibrary.K2_SetTimer` null "EndDay" 1.0)))

(fn `ClockUpdateTimer`
  (bind _result (`/Engine/EditorBlueprintResources/StandardMacros.DecrementInt` (`self.GameTime`))
    (:`  `
      (`/Game/Blueprints/UI/WBP_Clock.UpdateTime` (`/Game/Blueprints/UI/WBP_MainUI.WBP_Clock` (`self.PlayerUI`)) _result)
      (if (<= (`self.GameTime`) 0)
        (`KismetSystemLibrary.K2_ClearAndInvalidateTimerHandle` (`self.ClockTimer`))))))

(fn `DayFinished`
  (`KismetSystemLibrary.K2_ClearAndInvalidateTimerHandle` (`self.TotalDayTimer`))
  (`self.CheckForEndDay`))

(fn `DayStart`
  (`GameplayStatics.SetGlobalTimeDilation` 1.0)
  (`self.DayStarted`)
  (`KismetArrayLibrary.Array_Clear` (`self.MissionsDone`))
  (set `self.FishCollected` 0)
  (bind _output_get (set `self.GameTime` 6))
  (bind _returnvalue (`KismetSystemLibrary.K2_SetTimer` null "DayFinished" (`KismetMathLibrary.Conv_IntToDouble` _output_get)))
  (set `self.TotalDayTimer` _returnvalue)
  (bind _returnvalue_2 (`KismetSystemLibrary.K2_SetTimer` null "ClockUpdateTimer" 1.0 true))
  (set `self.ClockTimer` _returnvalue_2)
  (`/Game/Blueprints/UI/WBP_Clock.UpdateTime` (`/Game/Blueprints/UI/WBP_MainUI.WBP_Clock` (`self.PlayerUI`)) (`self.GameTime`))
  (`self.MissionSpawnerTimer`))

(fn `EndDay`
  (bind (_greatest _lowest) (`self.CalculateMostAndLeastMissiomTypes` (`self.MissionsDone`)))
  (bind _values (`BlueprintMapLibrary.Map_Values` (`/Game/Blueprints/UI/WBP_PenguinHeroes.EnumToHero` (`/Game/Blueprints/UI/WBP_MainUI.WBP_PenguinHeroes` (`self.PlayerUI`)))))
  (for _array_element _values
    (if (not (`/Game/Blueprints/UI/WBP_MissionPenguin.Locked` _array_element))
      (bind _returnvalue (- (`self.Fishes`) (+ (`/Game/Blueprints/UI/WBP_MissionPenguin.Level` _array_element) 1)))
      (if (< _returnvalue 0)
        (`/Game/Blueprints/UI/WBP_MissionPenguin.LockPenguin` _array_element)
        (else
          (set `self.Fishes` _returnvalue)))))
  (set `self.UsedFishes` (`self.GetPenguinCosts`))
  (`self.RehirePenguins`)
  (`GameplayStatics.SetGlobalTimeDilation` 0.0)
  (`/Game/Blueprints/UI/WBP_DayReview.Initialize` (`/Game/Blueprints/UI/WBP_MainUI.WBP_DayReview` (`self.PlayerUI`)) (make `/Game/Blueprints/Data/ST_DayData` (`KismetArrayLibrary.Array_Length` (`self.MissionsDone`)) _greatest _lowest (`self.FishCollected`) (`self.UsedFishes`) (`self.Fishes`))))

(fn `GetPenguinCosts`
  (returns (TotalCosts :type Integer))
  (locals (`L-TotalCost` :type Integer))
  (bind _values (`BlueprintMapLibrary.Map_Values` (`/Game/Blueprints/UI/WBP_PenguinHeroes.EnumToHero` (`/Game/Blueprints/UI/WBP_MainUI.WBP_PenguinHeroes` (`self.PlayerUI`)))))
  (for _array_element _values
    (if (not (`/Game/Blueprints/UI/WBP_MissionPenguin.Locked` _array_element))
      (set `local.L-TotalCost` (+ (`/Game/Blueprints/UI/WBP_MissionPenguin.Level` _array_element) (`local.L-TotalCost`) 1))))
  (return (`local.L-TotalCost`)))

(fn `GetRelation`
  (params (RelationsOf :type "/Game/Blueprints/Data/E_Masks Enum" :default "NewEnumerator0") (Target :type "/Game/Blueprints/Data/E_Masks Enum" :default "NewEnumerator0"))
  (returns (Relation :type "/Game/Blueprints/Data/E_Status Enum"))
  (bind (_hawk _owl _peacock _raven _tucan) (break `/Game/Blueprints/Data/ST_FactionStatus` (select `/Game/Blueprints/Data/E_Masks` (`local.RelationsOf`) :`NewEnumerator1` (`self.Hawk`) :`NewEnumerator2` (`self.Owl`) :`NewEnumerator3` (`self.Peacock`) :`NewEnumerator4` (`self.Raven`) :`NewEnumerator5` (`self.Tucan`))))
  (return (select `/Game/Blueprints/Data/E_Masks` (`local.Target`) :`NewEnumerator0` "NewEnumerator0" :`NewEnumerator1` _hawk :`NewEnumerator2` _owl :`NewEnumerator3` _peacock :`NewEnumerator4` _raven :`NewEnumerator5` _tucan)))

(fn `MissionCompleted`
  (params (MissionData :type "/Game/Blueprints/Data/ST_MissionData Structure"))
  (bind ((`MissionGiver_31_CCAE2BFC4D208B983846BFAD44B6B8F0` _missiongiver) (`MissionTarget_35_B064C9994A4F7CA83C9762BAEE1FF0B6` _missiontarget) (`MaskReward_21_D213BD704D1B4D27492928A8EFA8552C` _maskreward) (`FishReward_22_717EC73A48EE639AA4AC46B971F93B37` _fishreward)) (break `/Game/Blueprints/Data/ST_MissionData` MissionData))
  (`KismetArrayLibrary.Array_Add` (`self.MissionsDone`) _missiongiver)
  (set `self.Fishes` (+ _fishreward (`self.Fishes`)))
  (set `self.FishCollected` (+ _fishreward (`self.FishCollected`)))
  (`self.AddMasks` _maskreward)
  (`self.ChangeRelation` _missiongiver "NewEnumerator0" -1))

(fn `MissionSpawnerTimer`
  (if (`KismetSystemLibrary.K2_IsValidTimerHandle` (`self.TotalDayTimer`))
    (bind _returnvalue (`KismetSystemLibrary.K2_SetTimer` null "SpawnMission" (`KismetMathLibrary.RandomFloatInRange` 3.0 3.0)))
    (set `self.SpawnMissionTimer` _returnvalue)))

(fn `RandomlyChangeRelations`
  (for _index (range 5)
    (bind _returnvalue (select `int` _index :`0` (`self.Hawk`) :`1` (`self.Owl`) :`2` (`self.Peacock`) :`3` (`self.Raven`) :`4` (`self.Tucan`)))
    (bind (_hawk _owl _peacock _raven _tucan) (break `/Game/Blueprints/Data/ST_FactionStatus` _returnvalue))
    (`|VariableSetRef` _returnvalue (make `/Game/Blueprints/Data/ST_FactionStatus` (`self.CalculateRelationChange` _hawk) (`self.CalculateRelationChange` _owl) (`self.CalculateRelationChange` _peacock) (`self.CalculateRelationChange` _raven) (`self.CalculateRelationChange` _tucan)))))

(fn `RehirePenguins`
  (bind _values (`BlueprintMapLibrary.Map_Values` (`/Game/Blueprints/UI/WBP_PenguinHeroes.EnumToHero` (`/Game/Blueprints/UI/WBP_MainUI.WBP_PenguinHeroes` (`self.PlayerUI`)))))
  (for _array_element _values
    (bind _returnvalue (+ (`/Game/Blueprints/UI/WBP_MissionPenguin.Level` _array_element) 1))
    (if (>= (`self.Fishes`) _returnvalue)
      (set `self.Fishes` (- (`self.Fishes`) _returnvalue))
      (`/Game/Blueprints/UI/WBP_MissionPenguin.UnLockPenguin` _array_element))))

(fn `SpawnMission`
  (bind _missionspawners (`self.MissionSpawners`))
  (if (and (<= (`self.ActiveMissionCount`) 8) (`KismetSystemLibrary.K2_IsValidTimerHandle` (`self.TotalDayTimer`)))
    (`KismetArrayLibrary.Array_Shuffle` _missionspawners)
    (for _array_element _missionspawners
      (if (not (`/Game/Blueprints/WorldObjects/BP_MissionSpawner.HasMission` _array_element))
        (`/Game/Blueprints/WorldObjects/BP_MissionSpawner.SpawnMission` _array_element)
        (`|ExecutionSequence`
          (:`then_0`
            (break))
          (:`then_1`
            (`/Engine/EditorBlueprintResources/StandardMacros.IncrementInt` (`self.ActiveMissionCount`)
              (:`  `
                (`self.MissionSpawnerTimer`)))))))))

(fn `UserConstructionScript`)