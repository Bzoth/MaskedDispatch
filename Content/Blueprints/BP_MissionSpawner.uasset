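; BP_MissionSpawner shows a mission pop-up through its widget component and hides it when clicked.
; On BeginPlay it casts the hosted widget to WBP_MissionPopUp and binds to its PopupClicked event, which hides the component.
; After a short delay, SpawnMissionPopup unhides the component and plays a 2D sound, so the pop-up appears once, with no repeat spawning.
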(event `self.ReceiveBeginPlay`
  (`|ExecutionSequence`
    (:`then_0`
      (bind _aswbp_mission_pop_up (cast `/Game/Blueprints/WBP_MissionPopUp` (`WidgetComponent.GetWidget` (`self.Widget`))))
      (add `/Game/Blueprints/WBP_MissionPopUp.PopupClicked` _aswbp_mission_pop_up (delegate `PopupClicked_Event`)))
    (:`then_1`
      ;[0.15 0 0 0.5] Comment
      (`KismetSystemLibrary.Delay` 0.2)
      (`self.SpawnMissionPopup`))))

(event `PopupClicked_Event`
  (`SceneComponent.SetHiddenInGame` (`self.Widget`) true false))

(fn `SpawnMissionPopup`
  (`SceneComponent.SetHiddenInGame` (`self.Widget`) false false)
  (`GameplayStatics.SpawnSound2D` "/Engine/EditorSounds/Notifications/CompileSuccess.CompileSuccess" 1.0 1.0 0.0 null))

(fn `UserConstructionScript`)