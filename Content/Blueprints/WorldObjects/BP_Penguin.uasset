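; World actor for a penguin hero that travels to mission areas and back to base, with a popup image matching its stat type.
; SetMoveTarget and ReturnToBase set a destination that Tick approaches at constant speed, showing the popup widget during travel.
; Arrival hides the popup and fires ReachedEventArea, plus ReturnFromMission on the hero UI after a return.
; Each new target rebinds the mission area's SendPenguinBack event.
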(event `self.ReceiveBeginPlay`
  (bind _aswbp_penguin_popup (cast `/Game/Blueprints/UI/WBP_PenguinPopup` (`WidgetComponent.GetWidget` (`self.Widget`))))
  (set `self.Popup` _aswbp_penguin_popup))

(event `self.ReceiveTick`
  (params (DeltaSeconds :type "Float (single-precision)"))
  (if (`self.ShouldMove`)
    (`self.K2_SetActorLocation` (`KismetMathLibrary.VInterpTo_Constant` (`self.K2_GetActorLocation`) (`self.Destination`) DeltaSeconds 300.0))
    (if (== (`self.K2_GetActorLocation`) (`self.Destination`) :`ErrorTolerance` 1.0)
      (set `self.ShouldMove` false)
      (`self.ReachedEventArea` (`self.MissionData`) self)
      (`SceneComponent.SetHiddenInGame` (`self.Widget`) true false)
      (if (`self.IsReturningToBase`)
        (set `self.IsReturningToBase` false)
        (bind _returnvalue (`GameplayStatics.GetActorOfClass` "/Game/Blueprints/Managment/BP_GameManager.BP_GameManager_C"))
        (`/Game/Blueprints/UI/WBP_MissionPenguin.ReturnFromMission` (`BlueprintMapLibrary.Map_Find` (`/Game/Blueprints/UI/WBP_PenguinHeroes.EnumToHero` (`/Game/Blueprints/UI/WBP_MainUI.WBP_PenguinHeroes` (`/Game/Blueprints/Managment/BP_GameManager.PlayerUI` _returnvalue))) (`self.Penguins`)))))))

(fn `ReturnToBase`
  (set `self.IsReturningToBase` true)
  (set `self.ShouldMove` true)
  (set `self.Destination` (100.0 -120.0 -860.0))
  (`SceneComponent.SetHiddenInGame` (`self.Widget`) false false))

(fn `SetMoveTarget`
  (params (Destination :type "Vector Structure") (MissionData :type "/Game/Blueprints/Data/ST_MissionData Structure") (MissionArea :type "/Game/Blueprints/WorldObjects/BP_MissionSpawner Object Reference"))
  (bind _target (`self.Target`)
    (:`then`
      (clear `/Game/Blueprints/WorldObjects/BP_MissionSpawner.SendPenguinBack` _target))
    (:`else`
      _))
  (set `self.ShouldMove` true)
  (set `self.Destination` Destination)
  (set `self.MissionData` MissionData)
  (`SceneComponent.SetHiddenInGame` (`self.Widget`) false false)
  (bind _output_get (set `self.Target` MissionArea))
  (add `/Game/Blueprints/WorldObjects/BP_MissionSpawner.SendPenguinBack` _output_get (`|CreateDelegate` :!event `ReturnToBase`)))

(fn `SetPenguin`
  (params (Penguin :type "/Game/Blueprints/Data/E_Penguin Enum" :default "NewEnumerator0"))
  (set `self.Penguins` Penguin)
  (`/Game/Blueprints/UI/WBP_PenguinPopup.SetVisual` (`self.Popup`) (select `/Game/Blueprints/Data/E_Penguin` (`self.Penguins`) :`NewEnumerator0` "/Game/Assets/TexturesReel/T2D_Empty.T2D_Empty" :`NewEnumerator1` "/Game/Assets/TexturesReel/T2D_Penguin_CHA.T2D_Penguin_CHA" :`NewEnumerator2` "/Game/Assets/TexturesReel/T2D_Penguin_DEX.T2D_Penguin_DEX" :`NewEnumerator3` "/Game/Assets/TexturesReel/T2D_Penguin_INT.T2D_Penguin_INT" :`NewEnumerator4` "/Game/Assets/TexturesReel/T2D_Penguin_STR.T2D_Penguin_STR" :!type "Texture2D Object Reference")))

(fn `UserConstructionScript`)