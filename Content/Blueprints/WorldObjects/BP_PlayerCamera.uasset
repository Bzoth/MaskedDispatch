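; BP_PlayerCamera is the player camera Blueprint that sets up the main UI and a hold-to-fast-forward control.
; On BeginPlay it shows the mouse cursor, adds a WBP_MainUI widget to the viewport and hands it to the level's BP_GameManager as its PlayerUI.
; Holding Space raises global time dilation to speed up the game, and releasing it restores normal speed.
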(event `self.ReceiveBeginPlay`
  (`|ExecutionSequence`
    (:`then_0`
      (set `PlayerController.bShowMouseCursor` true (`GameplayStatics.GetPlayerController` 0)))
    (:`then_1`
      (bind _returnvalue (`|CreateWidget` "/Game/Blueprints/UI/WBP_MainUI.WBP_MainUI_C"))
      (bind _output_get (set `self.MainUI` _returnvalue))
      (`UserWidget.AddToViewport` _output_get 0))
    (:`then_2`
      (bind _returnvalue_2 (`GameplayStatics.GetActorOfClass` "/Game/Blueprints/Managment/BP_GameManager.BP_GameManager_C"))
      (set `/Game/Blueprints/Managment/BP_GameManager.PlayerUI` (`self.MainUI`) _returnvalue_2))))

(event `Key|SpaceBar`
  (params (Key :type "Key Structure"))
  (:`Pressed`
    (`GameplayStatics.SetGlobalTimeDilation` 10.0))
  (:`Released`
    (`GameplayStatics.SetGlobalTimeDilation` 1.0)))

(fn `UserConstructionScript`)